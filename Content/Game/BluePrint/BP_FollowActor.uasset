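; A magnetic physics object that the player pulls or pushes with magnet polarity, with a north or south mesh chosen from its pole at BeginPlay.
; On magnet interaction it applies attractive or repulsive force based on pole match, unless the player is within the minimum attraction distance.
; Falling below a height threshold teleports it to its start location and resets physics.
; Placement on a follow stand disables interaction and physics.
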(event Custom|OnPlacedOnFollowStand
  ;[0.15 0.15 0.15 0.5] スタンドに配置されたら
  (Variables|Default|SetCan%20Interact false)
  (Physics|SetSimulatePhysics (Variables|Default|GetStaticMesh) false))

(event EventTick
  (params (DeltaSeconds :type Float%20%28single-precision%29))
  (|CallParentFunction DeltaSeconds)
  (if (not (> (.Z (Math|Vector|BreakVector (Transformation|GetActorLocation self))) (Variables|Default|GetFall%20Death%20Threshold)))
    (Transformation|SetActorLocation (Variables|Default|GetReSpawn%20Position) false true)
    (Physics|SetSimulatePhysics (Variables|Default|GetStaticMesh) false)
    (Physics|SetSimulatePhysics (Variables|Default|GetStaticMesh) true)
    (Development|PrintString "ボールが落下しました")))

(event EventBeginPlay
  ;[0.15 0.15 0.15 0.5] スタート時スタティックメッシュの変更をする
  (Variables|Default|SetReSpawn%20Position (Transformation|GetActorLocation self))
  (switch Utilities|FlowControl|Switch|SwitchonEMagnetPole (Variables|Default|GetMagnetPole)
    (:NewEnumerator0
      (Components|StaticMesh|SetStaticMesh (Variables|Default|GetStaticMesh) "/Game/Assets/Object/SM_NorthMountainShapeCore.SM_NorthMountainShapeCore"))
    (:NewEnumerator1
      (Components|StaticMesh|SetStaticMesh (Variables|Default|GetStaticMesh) "/Game/Assets/Object/SM_SouthMoutainShapeCore.SM_SouthMoutainShapeCore")))
  (|CallParentFunction))

(event Collision|EventActorBeginOverlap
  (params (OtherActor :type Actor%20Object%20Reference))
  (|CallParentFunction OtherActor) ; このノードは無効になっているため呼び出せません。\n機能をビルドするにはピンをドラッグしてください。
)

(event EventMagnetInteract
  (params (Player%20Magnet%20Pole :type EMagnetPole%20Enum :default "NewEnumerator0") (Player :type Actor%20Object%20Reference) (Player%20Chara%20Movement :type Character%20Movement%20Component%20Object%20Reference) (Delta%20Time :type Float%20%28double-precision%29))
  ;[0.15 0.15 0.15 0.5] インタラクト時はある程度離れていれば近づく
  (Utilities|FlowControl|Sequence
    (:then_0
      (Rendering|Debug|DrawDebugSphere (Transformation|GetActorLocation Player) (Math|Conversions|ToFloat(Integer) (Variables|Default|GetMin%20Attractive%20Distance)) 8 "(R=1.000000,G=1.000000,B=1.000000,A=1.000000)" 0.1))
    (:then_1
      (if (not (CallFunction|IsDistanceNotOver(Actor) Player self (Variables|Default|GetMin%20Attractive%20Distance)))
        (Physics|AddForce (Variables|Default|GetStaticMesh) (CallFunction|GetDistancetoPlayer Player self (CallFunction|IsMagnetPoleEqual Player%20Magnet%20Pole) (Variables|Default|GetRepulsive%20Force) (Variables|Default|GetAttractive%20Force)) "None" false)))))

(fn ConstructionScript
  (|CallParentFunction))