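; BP_Wind is a wind zone actor that pushes the magnet character and fall blocks inside it.
; At BeginPlay it derives the wind vector from StartPoint to EndPoint and spawns the NS_Wind Niagara effect, sized from the collision bounds and driven by that vector.
; Overlap events track the character's movement component and other actors.
; Tick applies the scaled wind force to that component and to tracked BP_FallBlock meshes.
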(event EventBeginPlay
  (bind _collisioncomponent (Variables|Default|GetCollisionComponent))
  (bind _boxextent (Collision|GetComponentBounds _collisioncomponent))
  (bind _returnvalue (* _boxextent 2))
  (bind (_x _y _z) (Math|Vector|BreakVector _returnvalue))
  ;[1 0 0.8811 0.5] ゲーム開始時、風ベクトルを事前に計算して、Niagaraエフェクトに風の強さを代入
  (Variables|Default|SetWind%20Vector (- (Transformation|GetWorldLocation (Variables|Default|GetEndPoint)) (Transformation|GetWorldLocation (Variables|Default|GetStartPoint))))
  (bind _returnvalue_2 (Niagara|SpawnSystematLocation "/Game/Game/Niagara/NS_Wind.NS_Wind" (Transformation|GetWorldLocation (Variables|Default|GetParticle%20Pos)) (Transformation|GetActorRotation self) (Transformation|GetActorScale3D self)))
  (Utilities|FlowControl|Sequence
    (:then_0
      (Class|NiagaraComponent|SetVariableVec2 _returnvalue_2 "PlaneSize" (Math|Vector2D|MakeVector2D _z _y)))
    (:then_1
      (Niagara|SetNiagaraVariable(Vector3) _returnvalue_2 "WindVelocity" (Variables|Default|GetWind%20Vector)))))

(event EventTick
  (params (DeltaSeconds :type Float%20%28single-precision%29))
  (bind _playercharactermovement (Variables|Default|GetPlayerCharacterMovement))
  (bind _wind_vector (Variables|Default|GetWind%20Vector))
  (bind _returnvalue (* _wind_vector 200))
  ;[0.15 0.15 0.15 0.5] Tick内で(Start → End) × WindPowerの力だけWindowObjectsに力を加える(CharacterMovementは一度だけ実行する為DoOnce)
  (Utilities|FlowControl|Sequence
    (:then_0
      (Utilities|IsValid _playercharactermovement
        (:Is%20Valid
          (Physics|AddForce _playercharactermovement _returnvalue))))
    (:then_1
      (for _array_element (Variables|Default|GetWindowObjects)
        (bind _asbp_fall_block (Utilities|Casting|CastToBP_FallBlock _array_element))
        (Physics|AddForce (Variables|/Game/Game/BluePrint/BP_FallBlock.BP_FallBlock_C|GetStaticMesh _asbp_fall_block) _returnvalue "None" false)))))

(event Collision|EventActorBeginOverlap
  (params (OtherActor :type Actor%20Object%20Reference))
  ;[0.15 0.15 0.15 0.5] トリガーに出入りしたらCharacterMovementを取得。
  (bind _asbp_magnet_character (Utilities|Casting|CastToBP_MagnetCharacter OtherActor)
    (:then
      (Variables|Default|SetPlayerCharacterMovement (Variables|/Script/Engine.Character|GetCharacterMovement _asbp_magnet_character)))
    (:CastFailed
      (if (not (Utilities|Array|ContainsItem (Variables|Default|GetWindowObjects) _asbp_magnet_character))
        (Utilities|Array|Add (Variables|Default|GetWindowObjects) OtherActor)))))

(event Collision|EventActorEndOverlap
  (params (OtherActor :type Actor%20Object%20Reference))
  ;[0.15 0.15 0.15 0.5] トリガーに出入りしたらCharacterMovementを取得。
  (bind _asbp_magnet_character (Utilities|Casting|CastToBP_MagnetCharacter OtherActor)
    (:then
      (Variables|Default|SetPlayerCharacterMovement 0))
    (:CastFailed
      (if (Utilities|Array|ContainsItem (Variables|Default|GetWindowObjects) _asbp_magnet_character)
        (Utilities|Array|RemoveItem (Variables|Default|GetWindowObjects) OtherActor)))))

(fn ConstructionScript)