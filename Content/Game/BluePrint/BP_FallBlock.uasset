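; BP_FallBlock is a platform block that falls shortly after the player's BP_MagnetCharacter overlaps it, then respawns.
; A DoOnce-guarded overlap turns the mesh orange, waits WaitBlockTime, then enables physics simulation and calls ReSpawn.
; After a fixed delay, ReSpawn re-arms the trigger, teleports the block to its BeginPlay transform, disables physics and restores the yellow material.
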(event Custom|ReSpawn
  ;[0.15 0.15 0.15 0.5] プレイヤーが入ったら数秒後に重力が働き始めてブロックが消える
  ;;[0.15 0.15 0.15 0.5] 3秒待ってリスポーン処理を行う
  (Utilities|FlowControl|Delay 3.0)
  (Utilities|FlowControl|Sequence
    (:then_0
      (Utilities|FlowControl|DoOnce false) ; enters at Reset
    )
    (:then_1
      (Transformation|SetActorLocation self (Variables|Default|GetRestartPosition) false true)
      (Transformation|SetActorRotation (Variables|Default|GetRestartRotation) true)
      (Physics|SetSimulatePhysics (Variables|Default|GetStaticMesh) false)
      (Rendering|Material|SetMaterial (Variables|Default|GetStaticMesh) 0 "/Game/LevelPrototyping/Materials/MI_Solid_Materials/MI_Solid_Yellow.MI_Solid_Yellow"))))

(event EventBeginPlay
  (Variables|Default|SetRestartPosition (Transformation|GetActorLocation))
  (Variables|Default|SetRestartRotation (Transformation|GetActorRotation)))

(event Collision|EventActorBeginOverlap
  (params (OtherActor :type Actor%20Object%20Reference))
  ;[0.15 0.15 0.15 0.5] プレイヤーが入ったら数秒後に重力が働き始めてブロックが消える
  (Utilities|Casting|CastToBP_MagnetCharacter OtherActor)
  (Utilities|FlowControl|DoOnce false
    (:Completed
      (Rendering|Material|SetMaterial (Variables|Default|GetStaticMesh) 0 "/Game/LevelPrototyping/Materials/MI_Solid_Materials/MI_Solid_Orange.MI_Solid_Orange")
      (Utilities|FlowControl|Delay (Variables|Default|GetWait%20Block%20Time))
      (Physics|SetSimulatePhysics (Variables|Default|GetStaticMesh) true)
      (CallFunction|ReSpawn))))

(fn ConstructionScript)