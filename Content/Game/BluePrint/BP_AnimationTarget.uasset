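; BP_AnimationTarget is a magnetic target actor that plays level sequence animations in response to the player's magnet.
; MagnetInteract compares poles, triggering the repulsive sequence when they match and the attractive one otherwise, if that sequence is valid.
; BeginPlay sets the North or South core mesh from MagnetPole.
; ReversePole queues the opposite mesh in NextCoreStaticMesh, then hands off to the parent class's pole reversal.
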(event EventBeginPlay
  (switch Utilities|FlowControl|Switch|SwitchonEMagnetPole (Variables|Default|GetMagnetPole)
    (:NewEnumerator0
      (Components|StaticMesh|SetStaticMesh (Variables|Default|GetStaticMesh) "/Game/Assets/Object/SM_NorthMountainShapeCore.SM_NorthMountainShapeCore"))
    (:NewEnumerator1
      (Components|StaticMesh|SetStaticMesh (Variables|Default|GetStaticMesh) "/Game/Assets/Object/SM_SouthMoutainShapeCore.SM_SouthMoutainShapeCore")))
  (|CallParentFunction))

(event Collision|EventActorBeginOverlap
  (params (OtherActor :type Actor%20Object%20Reference))
  (|CallParentFunction OtherActor) ; このノードは無効になっているため呼び出せません。\n機能をビルドするにはピンをドラッグしてください。
)

(event EventReversePole
  ;[0 0.06231 0.8156 0.5] 極変更の際コアの部分のスタティックメッシュを変更する
  (switch Utilities|FlowControl|Switch|SwitchonEMagnetPole (Variables|Default|GetMagnetPole)
    (:NewEnumerator0
      (Variables|Default|SetNext%20Core%20StaticMesh "/Game/Assets/Object/SM_SouthMoutainShapeCore.SM_SouthMoutainShapeCore"))
    (:NewEnumerator1
      (Variables|Default|SetNext%20Core%20StaticMesh "/Game/Assets/Object/SM_NorthMountainShapeCore.SM_NorthMountainShapeCore")))
  (|CallParentFunction))

(event EventMagnetInteract
  (params (Player%20Magnet%20Pole :type EMagnetPole%20Enum :default "NewEnumerator0") (Player :type Actor%20Object%20Reference) (Player%20Chara%20Movement :type Character%20Movement%20Component%20Object%20Reference) (Delta%20Time :type Float%20%28double-precision%29))
  (bind _replusive_levelsequence (Variables|Default|GetReplusive%20LevelSequence))
  (bind _attractive_levelsequence (Variables|Default|GetAttractive%20LevelSequence))
  ;[0.5729 0.02068 0 0.5] 極にあったアニメーションを再生するよってやつ
  (if (CallFunction|IsMagnetPoleEqual Player%20Magnet%20Pole)
    (Utilities|IsValid _replusive_levelsequence
      (:Is%20Valid
        (Class|MovieSceneSequencePlayer|Playto _replusive_levelsequence (Utilities|Struct|MakeMovieSceneSequencePlaybackParams "(FrameNumber=(Value=0),SubFrame=0.000000)" 0.0 "Start" "(Hours=0,Minutes=0,Seconds=0,Frames=0,Subframe=0.000000,bDropFrameFormat=False)" "MarkedFrame" "Play"))))
    (else
      (Utilities|IsValid _attractive_levelsequence
        (:Is%20Valid
          (Class|MovieSceneSequencePlayer|Playto _attractive_levelsequence (Utilities|Struct|MakeMovieSceneSequencePlaybackParams "(FrameNumber=(Value=0),SubFrame=0.000000)" 0.0 "End" "(Hours=0,Minutes=0,Seconds=0,Frames=0,Subframe=0.000000,bDropFrameFormat=False)" "MarkedFrame" "Play")))))))

(fn ConstructionScript
  (|CallParentFunction))