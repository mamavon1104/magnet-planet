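; BP_Lever is a magnet-polarity lever that responds only when the interacting player's pole differs from its own.
; Interaction calls the pole-change start and plays or reverses a rotation Timeline; finishing flips the pole, swapping ring material and lever mesh.
; A DoOnce, reset after a post-flip delay, blocks retriggering, and BeginPlay also runs the Timeline branch.
; A looping timer uses a cross product to turn the cursor pivot according to the player's side.
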(event Custom|Check%20Is%20Hit%20Ray%20Cast
  (Utilities|IsValid (Variables|Default|GetPlayer)
    (:Is%20Valid
      ;[0.15 0.15 0.15 0.5] zベクトルの外積結果で左右か確認
      (if (< (.Z (Math|Vector|BreakVector (.Cross (CallFunction|GetTargetandForwardDotCross(Actor) (Variables|Default|GetPlayer) self)))) 0.0)
        ;[0.15 0.15 0.15 0.5] 右の場合
        (Transformation|SetRelativeRotation (Variables|Default|GetCursor%20Pivot) "0, 0, 0" false false)
        (else
          ;[0.15 0.15 0.15 0.5] 左の場合
          (Transformation|SetRelativeRotation (Variables|Default|GetCursor%20Pivot) "0.000000,180.000000,0.000000" false false))))))

(event Custom|Animation%20Finished
  (Utilities|FlowControl|DoOnce false) ; enters at Reset
)

(event EventBeginPlay
  (Utilities|Time|SetTimerbyEvent (delegate Custom|Check%20Is%20Hit%20Ray%20Cast) 0.5 true)
  (|CallParentFunction)
  ;[0.15 0.15 0.15 0.5] 自分を回転させるだけのタイムライン、終わったら磁極が反転するように
  (switch Utilities|FlowControl|Switch|SwitchonEMagnetPole (Variables|Default|GetMagnetPole)
    (:NewEnumerator0
      (bind _lever_rotation (Timeline|タイムライン Play)
        (:Update
          (Transformation|SetRelativeRotation (Variables|Default|GetSM_Lever) (Math|Rotator|MakeRotator 0.0 _lever_rotation 0.0) false false))
        (:Finished
          (Default|ReversePole self)
          (Utilities|FlowControl|Delay 5.0)
          (CallFunction|AnimationFinished))))
    (:NewEnumerator1
      (Timeline|タイムライン Reverse))))

(event Collision|EventActorBeginOverlap
  (params (OtherActor :type Actor%20Object%20Reference))
  (|CallParentFunction OtherActor) ; このノードは無効になっているため呼び出せません。\n機能をビルドするにはピンをドラッグしてください。
)

(event EventTick
  (params (DeltaSeconds :type Float%20%28single-precision%29)))

(event EventReversePole
  (|CallParentFunction)
  (switch Utilities|FlowControl|Switch|SwitchonEMagnetPole (Variables|Default|GetMagnetPole)
    (:NewEnumerator0
      (Rendering|Material|SetMaterial (Variables|Default|GetStaticMesh) 0 "/Game/Assets/Object/MI_RedRing.MI_RedRing")
      (Components|StaticMesh|SetStaticMesh (Variables|Default|GetSM_Lever) "/Game/Assets/SM_NorthLever.SM_NorthLever"))
    (:NewEnumerator1
      (Rendering|Material|SetMaterial (Variables|Default|GetStaticMesh) 0 "/Game/Assets/Object/MI_RingBlue.MI_RingBlue")
      (Components|StaticMesh|SetStaticMesh (Variables|Default|GetSM_Lever) "/Game/Assets/SM_SouthLever.SM_SouthLever"))))

(event EventMagnetInteract
  (params (Player%20Magnet%20Pole :type EMagnetPole%20Enum :default "NewEnumerator0") (Player :type Actor%20Object%20Reference) (Player%20Chara%20Movement :type Character%20Movement%20Component%20Object%20Reference) (Delta%20Time :type Float%20%28double-precision%29))
  ;[0.15 0.15 0.15 0.5] 別の極の場合のみレバーインタラクトとして認識するよ
  (Utilities|IsValid (Variables|Default|GetPlayer)
    (:Is%20Valid
      (if (not (CallFunction|IsMagnetPoleEqual Player%20Magnet%20Pole))
        (Utilities|FlowControl|DoOnce false
          (:Completed
            ;[0 0.7865 0.1606 0.5] ここで極変更って訳
            (Default|CallStartChangePole)
            ;[0.15 0.15 0.15 0.5] 自分を回転させるだけのタイムライン、終わったら磁極が反転するように
            (switch Utilities|FlowControl|Switch|SwitchonEMagnetPole (Variables|Default|GetMagnetPole)
              (:NewEnumerator0
                (bind _lever_rotation (Timeline|タイムライン Play)
                  (:Update
                    (Transformation|SetRelativeRotation (Variables|Default|GetSM_Lever) (Math|Rotator|MakeRotator 0.0 _lever_rotation 0.0) false false))
                  (:Finished
                    (Default|ReversePole self)
                    (Utilities|FlowControl|Delay 5.0)
                    (CallFunction|AnimationFinished))))
              (:NewEnumerator1
                (Timeline|タイムライン Reverse)))))))
    (:Is%20Not%20Valid
      (Variables|Default|SetPlayer Player))))

(fn ConstructionScript
  (|CallParentFunction))