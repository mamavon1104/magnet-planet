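; Function library of actor helpers, apparently for a magnet-based interaction mechanic.
; Two functions build large force vectors along the object-player axis or an object's forward axis, with a bool choosing sign and multiplier.
; Distance checks test whether two positions or actors lie within a range.
; A hit filter collects unique interactable BP_MagnetInteractableBase actors and reports whether any were found.
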(fn GetDistancetoPlayer
  (params (Player%20Actor :type Actor%20Object%20Reference) (Object%20Actor :type Actor%20Object%20Reference) (Is%20Object%20To%20Player :type Boolean) (To%20Object%20%20Force :type Float%20%28double-precision%29) (To%20Player%20Force :type Float%20%28double-precision%29))
  (bind _returnvalue (Transformation|GetActorLocation Object%20Actor))
  (bind _returnvalue_2 (Transformation|GetActorLocation Player%20Actor))
  (bind _returnvalue_3 (- _returnvalue_2 _returnvalue))
  (bind _returnvalue_4 (Math|Vector|Normalize _returnvalue_3))
  ;[0.624 0.4912 0.05767 0.5] (プレイヤー - オブジェクト)距離を正規化
  (if Is%20Object%20To%20Player
    ;[0.1226 0.9615 0 0.5] True処理の場合は オブジェクト→プレイヤー
    (return (* _returnvalue_4 -100000 To%20Object%20%20Force))
    (else
      ;[0.9615 0.04563 0 0.5] False処理の場合は プレイヤー→オブジェクト
      (return (* To%20Player%20Force 100000 _returnvalue_4)))))

(fn IsDistanceNotOver(Position)
  (params (Object%201 :type Vector) (Object2 :type Vector) (Distance :type Integer))
  ;[0.15 0.15 0.15 0.5] 2つのオブジェクトの距離を求めて Distance以内だったらtrueを返す
  (return (<= (Math|Vector|Distance(Vector) Object%201 Object2) Distance)))

(fn IsDistanceNotOver(Actor)
  (params (Object%201 :type Actor%20Object%20Reference) (Object2 :type Actor%20Object%20Reference) (Distance :type Integer))
  ;[0.15 0.15 0.15 0.5] 2つのオブジェクトの距離を求めて Distance以内だったらtrueを返す
  (return (<= (Math|Vector|Distance(Vector) (Transformation|GetActorLocation Object%201) (Transformation|GetActorLocation Object2)) Distance)))

(fn GetInteractableActorinHits
  (params (HitActors :type Array%20of%20Hit%20Result%20Structures))
  (bind _returnvalue (LocalVariables|GetReturnValue))
  ;[0.15 0.15 0.15 0.5] インタラクト可能なオブジェクトをひたすら配列の中に詰めていくよ
  (for _array_element HitActors
    (bind _asbp_magnet_interactable_base (Utilities|Casting|CastToBP_MagnetInteractableBase (.HitActor (Collision|BreakHitResult _array_element))))
    (if (Variables|/Game/Game/BluePrint/Base/BP_MagnetInteractableBase.BP_MagnetInteractableBase_C|GetCan%20Interact _asbp_magnet_interactable_base)
      (if (not (Utilities|Array|ContainsItem (LocalVariables|GetReturnValue) _asbp_magnet_interactable_base))
        (Utilities|Array|Add (LocalVariables|GetReturnValue) _asbp_magnet_interactable_base))))
  (return (Utilities|Array|IsValidIndex _returnvalue) _returnvalue))

(fn GetXVector
  (params (Object%20Actor :type Actor%20Object%20Reference) (Is%20Object%20To%20Player :type Boolean) (To%20Forward%20Force :type Float%20%28double-precision%29) (To%20Back%20Force :type Float%20%28double-precision%29))
  (bind _returnvalue (Transformation|GetActorForwardVector Object%20Actor))
  ;[0.624 0.4912 0.05767 0.5] オブジェクト前方ベクトルを取得
  (if Is%20Object%20To%20Player
    ;[0.1226 0.9615 0 0.5] True処理の場合は Forwardベクトル
    (return (* _returnvalue -100000 To%20Forward%20Force))
    (else
      ;[0.9615 0.04563 0 0.5] False処理の場合は backベクトル
      (return (* To%20Back%20Force 100000 _returnvalue)))))