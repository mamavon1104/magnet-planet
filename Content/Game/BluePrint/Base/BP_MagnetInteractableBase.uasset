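; Base Blueprint for magnet-interactable actors, holding a North/South pole and showing a targeting cursor when a player's ray hits it.
; Ray hit and miss events toggle the cursor widget's visibility; while visible, Tick orients its pivot along the player-to-cursor direction and spins the widget on roll.
; ReversePole flips the pole and spawns a red or blue Niagara effect.
; A helper compares poles; MagnetInteract is an empty event here.
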(event Custom|Reverse%20Pole
  (bind _self self)
  (bind _returnvalue (Transformation|GetActorLocation _self))
  ;[0.15 0.15 0.15 0.5] コメント
  (bind _output_get (Variables|Default|SetMagnetPole (CallFunction|ReturnReversePole)))
  (switch Utilities|FlowControl|Switch|SwitchonEMagnetPole _output_get
    (:NewEnumerator0
      (Niagara|SpawnSystematLocation "/Game/Game/Niagara/NS_ChangePoleRed.NS_ChangePoleRed" _returnvalue))
    (:NewEnumerator1
      (Niagara|SpawnSystematLocation "/Game/Game/Niagara/NS_ChangePoleBlue.NS_ChangePoleBlue" _returnvalue))))

(event EventBeginPlay
  ;[0.15 0.15 0.15 0.5] スタート時とレイヒットとレイを外したときにVisibilityの変更をして、
  ; Rayが当たっている時だけは回転も算出する。
  (Widget|SetVisibility (UserInterface|GetUserWidgetObject (Variables|Default|GetCursorWidget)) (CallFunction|GetVisibility (Variables|Default|GetDraw%20Cursor))))

(event Collision|EventActorBeginOverlap
  (params (OtherActor :type Actor%20Object%20Reference)))

(event EventMagnetInteract
  (params (Player%20Magnet%20Pole :type EMagnetPole%20Enum :default "NewEnumerator0") (Player :type Actor%20Object%20Reference) (Player%20Chara%20Movement :type Character%20Movement%20Component%20Object%20Reference) (Delta%20Time :type Float%20%28double-precision%29))
  ;[0.15 0.15 0.15 0.5] 今のEnumと等しいかをチェックしてイベント送信
)

(event EventHitRayEventCursor
  (params (Player :type Actor%20Object%20Reference))
  ;[0.15 0.15 0.15 0.5] スタート時とレイヒットとレイを外したときにVisibilityの変更をして、
  ; Rayが当たっている時だけは回転も算出する。
  (bind _output_get (Variables|Default|SetDraw%20Cursor true))
  (Variables|Default|SetPlayer%20Actor Player)
  (Development|PrintString (Utilities|String|ToString(Boolean) _output_get) true true "(R=0.000000,G=0.337420,B=1.000000,A=1.000000)")
  (Widget|SetVisibility (UserInterface|GetUserWidgetObject (Variables|Default|GetCursorWidget)) (CallFunction|GetVisibility (Variables|Default|GetDraw%20Cursor))))

(event EventMissRayEventCursor
  ;[0.15 0.15 0.15 0.5] スタート時とレイヒットとレイを外したときにVisibilityの変更をして、
  ; Rayが当たっている時だけは回転も算出する。
  (bind _output_get (Variables|Default|SetDraw%20Cursor false))
  (Development|PrintString (Utilities|String|ToString(Boolean) _output_get) true true "(R=1.000000,G=0.000000,B=0.060954,A=1.000000)")
  (Widget|SetVisibility (UserInterface|GetUserWidgetObject (Variables|Default|GetCursorWidget)) (CallFunction|GetVisibility (Variables|Default|GetDraw%20Cursor))))

(event EventTick
  (params (DeltaSeconds :type Float%20%28single-precision%29))
  (bind _cursorwidget (Variables|Default|GetCursorWidget))
  (bind _returnvalue (Transformation|GetWorldRotation _cursorwidget))
  (bind (_roll _pitch _yaw) (Math|Rotator|BreakRotator _returnvalue))
  ;[0.15 0.15 0.15 0.5] EventTickでカーソルの回転などを実装しています
  (if (Variables|Default|GetDraw%20Cursor)
    (Transformation|SetWorldRotation (Variables|Default|GetCursor%20Pivot) (Math|Rotator|FindLookatRotation (Transformation|GetActorLocation (Variables|Default|GetPlayer%20Actor)) (Transformation|GetWorldLocation (Variables|Default|GetCursor%20Pivot))) false false)
    (Transformation|SetWorldRotation (Variables|Default|GetCursorWidget) (Math|Rotator|MakeRotator (+ _roll -1.0) _pitch _yaw) false false)))

(fn ConstructionScript)

(fn IsMagnetPoleEqual
  (params (A :type Byte))
  (return (== A (Math|Conversions|ToInteger(Byte) (Variables|Default|GetMagnetPole)))))

(fn ReturnReversePole
  (switch Utilities|FlowControl|Switch|SwitchonEMagnetPole (Variables|Default|GetMagnetPole)
    (:NewEnumerator0
      (return "NewEnumerator1"))
    (:NewEnumerator1
      (return "NewEnumerator0"))))