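; BP_SwingTarget is a magnetic anchor whose North or South pole sets its sphere core mesh.
; MagnetInteract applies a force to the player from its pole comparison and attractive or repulsive strength, drawing a debug sphere for the release radius.
; Inside that radius, it resets the player's velocity and releases the player's opposite-pole object.
; ReversePole picks the opposite core mesh before handing off to parent logic.
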(event EventBeginPlay
  (switch Utilities|FlowControl|Switch|SwitchonEMagnetPole (Variables|Default|GetMagnetPole)
    (:NewEnumerator0
      (Components|StaticMesh|SetStaticMesh (Variables|Default|GetStaticMesh) "/Game/Assets/Object/SM_NorthSphereCore.SM_NorthSphereCore"))
    (:NewEnumerator1
      (Components|StaticMesh|SetStaticMesh (Variables|Default|GetStaticMesh) "/Game/Assets/Object/SM_SouthSphereCore.SM_SouthSphereCore")))
  (|CallParentFunction))

(event Collision|EventActorBeginOverlap
  (params (OtherActor :type Actor%20Object%20Reference))
  (|CallParentFunction OtherActor) ; このノードは無効になっているため呼び出せません。\n機能をビルドするにはピンをドラッグしてください。
)

(event EventReversePole
  ;[0 0.06231 0.8156 0.5] 極変更の際コアの部分のスタティックメッシュを変更する
  (switch Utilities|FlowControl|Switch|SwitchonEMagnetPole (Variables|Default|GetMagnetPole)
    (:NewEnumerator0
      (Variables|Default|SetNext%20Core%20StaticMesh "/Game/Assets/Object/SM_SouthSphereCore.SM_SouthSphereCore"))
    (:NewEnumerator1
      (Variables|Default|SetNext%20Core%20StaticMesh "/Game/Assets/Object/SM_NorthSphereCore.SM_NorthSphereCore")))
  (|CallParentFunction))

(event EventMagnetInteract
  (params (Player%20Magnet%20Pole :type EMagnetPole%20Enum :default "NewEnumerator0") (Player :type Actor%20Object%20Reference) (Player%20Chara%20Movement :type Character%20Movement%20Component%20Object%20Reference) (Delta%20Time :type Float%20%28double-precision%29))
  ;[0.5729 0.02068 0 0.5] プレイヤーをオブジェクトに引き寄せて、 指定した範囲内ならばプレイヤーの持っているオブジェクトをリリースする
  (Utilities|FlowControl|Sequence
    (:then_0
      ;[0.15 0.15 0.15 0.5] 球体のデバッグ、どれくらいの距離か分かりやすくするため
      (Rendering|Debug|DrawDebugSphere (Transformation|GetActorLocation self) (Math|Conversions|ToFloat(Integer) (Variables|Default|GetRelease%20Sphere%20Radius)) 4 "(R=0.000000,G=0.189954,B=1.000000,A=1.000000)" 0.0))
    (:then_1
      (Physics|AddForce Player%20Chara%20Movement (* (CallFunction|GetDistancetoPlayer Player self (CallFunction|IsMagnetPoleEqual Player%20Magnet%20Pole) (Variables|Default|GetRepulsive%20Force) (Variables|Default|GetAttractive%20Force)) -1))
      (if (CallFunction|IsDistanceNotOver(Actor) Player self (Variables|Default|GetRelease%20Sphere%20Radius))
        (bind _asbp_magnet_character (Utilities|Casting|CastToBP_MagnetCharacter Player))
        (Default|ResetVelocity _asbp_magnet_character)
        (switch Utilities|FlowControl|Switch|SwitchonEMagnetPole (Variables|Default|GetMagnetPole)
          (:NewEnumerator0
            (Default|ReleaseSouthObject _asbp_magnet_character))
          (:NewEnumerator1
            (Default|ReleaseNorthObject _asbp_magnet_character)))))))

(fn ConstructionScript
  (|CallParentFunction))