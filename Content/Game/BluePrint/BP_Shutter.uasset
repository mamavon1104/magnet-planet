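; BP_Shutter is a shutter whose vertical position is driven by a magnet interaction.
; On BeginPlay it caches the Shutter component's initial relative location.
; MagnetAlphaInteract uses the incoming alpha to interpolate relative Z from that start height to zero, keeping X and Y fixed and moving without sweep.
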(event EventMagnetAlphaInteract
  (params (NewParam :type Float%20%28double-precision%29))
  (bind _firstvector3pos (Variables|Default|GetFirstVector3Pos))
  (bind (_x _y _z) (Math|Vector|BreakVector _firstvector3pos))
  (Transformation|SetRelativeLocation (Variables|Default|GetShutter) (Math|Vector|MakeVector _x _y (Math|Float|Lerp _z 0.0 NewParam)) false false))

(event EventBeginPlay
  (Variables|Default|SetFirstVector3Pos (.Location (Math|Transform|BreakTransform (Transformation|GetRelativeTransform (Variables|Default|GetShutter))))))

(fn ConstructionScript)