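; A tutorial-style movie board actor that plays a video when BP_MagnetCharacter overlaps it.
; On overlap it opens and plays the MediaSource while a timeline scales up and spins the board in; leaving closes the media and reverses the timeline.
; While overlapped, Tick smoothly yaws the board to follow the player's position using a look-at rotation and RInterpTo.
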(event Collision|EventActorBeginOverlap
  (params (OtherActor :type Actor%20Object%20Reference))
  (bind _media_player (Variables|Default|GetMedia%20Player))
  (bind _asbp_magnet_character (Utilities|Casting|CastToBP_MagnetCharacter OtherActor))
  (Variables|Default|SetPlayer%20Character _asbp_magnet_character)
  (Variables|Default|SetIs%20Overlapping true)
  (Media|MediaPlayer|OpenSource _media_player (Variables|Default|GetMedia%20Source))
  (Media|MediaPlayer|Play _media_player :!class /Script/MediaAssets.MediaPlayer)
  (bind _openboard_alpha (Timeline|Open%20MovieBoard Play)
    (:Update
      (Transformation|SetRelativeScale3D (Variables|Default|GetSM_NaviBoard) (* (Math|Vector|MakeVector _openboard_alpha _openboard_alpha _openboard_alpha) 1.9))
      (Transformation|SetWorldRotation (Variables|Default|GetSM_NaviBoard) (Math|Rotator|Lerp(Rotator) (Transformation|GetWorldRotation (Variables|Default|GetSM_NaviBoard)) "0.000000,360.000000,0.000000" _openboard_alpha) false false))))

(event EventTick
  (params (DeltaSeconds :type Float%20%28single-precision%29))
  (if (Variables|Default|GetIs%20Overlapping)
    (Transformation|SetWorldRotation (Variables|Default|GetSM_NaviBoard) (Math|Interpolation|RInterpTo (Transformation|GetWorldRotation (Variables|Default|GetSM_NaviBoard)) (Math|Rotator|MakeRotator 0.0 0.0 (.Yaw (Math|Rotator|BreakRotator (Math|Rotator|FindLookatRotation (Transformation|GetActorLocation (Variables|Default|GetPlayer%20Character)) (Transformation|GetWorldLocation (Variables|Default|GetSM_NaviBoard)))))) DeltaSeconds 3.0) false false)))

(event Collision|EventActorEndOverlap
  (params (OtherActor :type Actor%20Object%20Reference))
  (Utilities|Casting|CastToBP_MagnetCharacter OtherActor)
  (Variables|Default|SetPlayer%20Character 0)
  (Variables|Default|SetIs%20Overlapping false)
  (Media|MediaPlayer|Close (Variables|Default|GetMedia%20Player) :!class /Script/MediaAssets.MediaPlayer)
  (bind _openboard_alpha (Timeline|Open%20MovieBoard Reverse)
    (:Update
      (Transformation|SetRelativeScale3D (Variables|Default|GetSM_NaviBoard) (* (Math|Vector|MakeVector _openboard_alpha _openboard_alpha _openboard_alpha) 1.9))
      (Transformation|SetWorldRotation (Variables|Default|GetSM_NaviBoard) (Math|Rotator|Lerp(Rotator) (Transformation|GetWorldRotation (Variables|Default|GetSM_NaviBoard)) "0.000000,360.000000,0.000000" _openboard_alpha) false false))))

(fn ConstructionScript)