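; Trigger actor that shows navigation text when BP_MagnetCharacter walks into it.
; On overlap it stores the player and passes its text, character reveal interval and view time to the character's DrawNavigateText, with an IsDoOnce option and a debug print.
; While the player stays inside, Tick smoothly turns the Board component to face them on yaw only.
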(event Collision|EventActorBeginOverlap
  (params (OtherActor :type Actor%20Object%20Reference))
  (Variables|Default|SetIs%20Player%20Overlapping true)
  (bind _asbp_magnet_character (Utilities|Casting|CastToBP_MagnetCharacter OtherActor))
  (if (Variables|Default|GetIs%20Do%20Once)
    (Utilities|FlowControl|DoOnce false
      (:Completed
        _)))
  (Variables|Default|SetPlayer _asbp_magnet_character)
  (Default|DrawNavigateText _asbp_magnet_character (Variables|Default|GetCharaInterval) (Variables|Default|GetTextInfo) (Variables|Default|GetView%20Time))
  (Development|PrintString "エリアに入ったのでテキスト表示アニメーション"))

(event Collision|EventActorEndOverlap
  (params (OtherActor :type Actor%20Object%20Reference))
  (Utilities|Casting|CastToBP_MagnetCharacter OtherActor)
  (Variables|Default|SetIs%20Player%20Overlapping false))

(event EventTick
  (params (DeltaSeconds :type Float%20%28single-precision%29))
  (if (Variables|Default|GetIs%20Player%20Overlapping)
    (Transformation|SetWorldRotation (Variables|Default|GetBoard) (Math|Interpolation|RInterpTo (Transformation|GetWorldRotation (Variables|Default|GetBoard)) (Math|Rotator|MakeRotator 0.0 0.0 (.Yaw (Math|Rotator|BreakRotator (Math|Rotator|FindLookatRotation (Transformation|GetWorldLocation (Variables|Default|GetBoard)) (Transformation|GetActorLocation (Variables|Default|GetPlayer)))))) DeltaSeconds 3.0) false false)))

(fn ConstructionScript)