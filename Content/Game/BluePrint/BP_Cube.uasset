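; BP_Cube is a magnetic cube with a north or south pole that the player's magnet can push or pull.
; On BeginPlay it sets the north or south core material from its pole, then runs the parent BeginPlay.
; On MagnetInteract it compares poles and feeds the result, with repulsive and attractive strengths, into GetDistanceToPlayer, applying the returned force to its static mesh through physics.
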(event EventBeginPlay
  (switch Utilities|FlowControl|Switch|SwitchonEMagnetPole (Variables|Default|GetMagnetPole)
    (:NewEnumerator0
      (Rendering|Material|SetMaterial (Variables|Default|GetStaticMesh) 0 "/Game/Assets/Object/MI_NorthCore.MI_NorthCore"))
    (:NewEnumerator1
      (Rendering|Material|SetMaterial (Variables|Default|GetStaticMesh) 0 "/Game/Assets/Object/MI_SouthCore.MI_SouthCore")))
  (|CallParentFunction))

(event EventMagnetInteract
  (params (Player%20Magnet%20Pole :type EMagnetPole%20Enum :default "NewEnumerator0") (Player :type Actor%20Object%20Reference) (Player%20Chara%20Movement :type Character%20Movement%20Component%20Object%20Reference) (Delta%20Time :type Float%20%28double-precision%29))
  (Physics|AddForce (Variables|Default|GetStaticMesh) (CallFunction|GetDistancetoPlayer Player self (CallFunction|IsMagnetPoleEqual Player%20Magnet%20Pole) (Variables|Default|GetRepulsive%20Force) (Variables|Default|GetAttractive%20Force)) "None" false))

(fn ConstructionScript)