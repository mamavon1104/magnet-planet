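; Player controller for the magnet character that handles respawning and timed camera cutaways.
; On UnPossess it prints a debug string, waits a tick, then spawns and possesses a new BP_MagnetCharacter at a player start.
; ChangeCameraPosition disables character movement and blends the view to a given target.
; After a delay it starts blending back to a temporary actor at the pawn's transform, immediately destroys it and restores walking.
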(event Custom|ChangeCameraPosition
  (params (CameraPosition :type Actor%20Object%20Reference) (Camera%20Move%20Time :type Float%20%28double-precision%29) (Delay%20Return%20TIme :type Float%20%28double-precision%29))
  (bind _self self)
  (bind _returnvalue (Pawn|GetControlledPawn _self))
  (bind _asbp_magnet_character (Utilities|Casting|CastToBP_MagnetCharacter _returnvalue))
  (Default|ChangeMovementState _asbp_magnet_character "MOVE_None")
  (bind _returnvalue_2 (Game|SpawnActorfromClass "/Script/Engine.Actor" (Transformation|GetActorTransform _returnvalue) "Undefined" "MultiplyWithRoot" 0 0))
  (Utilities|FlowControl|Sequence
    (:then_0
      (Game|Player|SetViewTargetwithBlend CameraPosition Camera%20Move%20Time "VTBlend_EaseInOut" 2.0 false))
    (:then_1
      (Utilities|FlowControl|Delay Delay%20Return%20TIme)
      (Game|Player|SetViewTargetwithBlend _returnvalue_2 Camera%20Move%20Time "VTBlend_EaseInOut" 2.0 false)
      (Actor|DestroyActor _returnvalue_2)
      (bind _asbp_magnet_character_2 (Utilities|Casting|CastToBP_MagnetCharacter (Pawn|GetControlledPawn self)))
      (Default|ChangeMovementState _asbp_magnet_character_2 "MOVE_Walking"))))

(event EventUnPossess
  (params (UnpossessedPawn :type Pawn%20Object%20Reference))
  (Development|PrintString "Hello")
  (Utilities|FlowControl|DelayUntilNextTick)
  (bind _returnvalue (Game|SpawnActorfromClass "/Game/Game/BluePrint/Character/BP_MagnetCharacter.BP_MagnetCharacter_C" (Transformation|GetActorTransform (Class|GameModeBase|FindPlayerStart (Game|GetGameMode) self)) "Undefined" "MultiplyWithRoot" 0 0))
  (Pawn|Possess self _returnvalue))

(fn ConstructionScript)