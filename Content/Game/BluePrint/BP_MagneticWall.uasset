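; Magnetic wall actor that pushes or pulls the player along an axis, depending on magnet polarity.
; BeginPlay sets the North or South core material from its pole, while Tick spins a cursor pivot.
; MagnetInteract box-traces forward over the interact length, sized from mesh scale, and on any hit applies repulsive or attractive force to the player's movement component based on pole match.
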(event EventTick
  (params (DeltaSeconds :type Float%20%28single-precision%29))
  (bind _cursor_pivot (Variables|Default|GetCursor%20Pivot))
  (bind _relativerotation (Variables|/Script/Engine.SceneComponent|GetRelativeRotation _cursor_pivot))
  (bind (_roll _pitch _yaw) (Math|Rotator|BreakRotator _relativerotation))
  (Transformation|SetRelativeRotation (Variables|Default|GetCursor%20Pivot) (Math|Rotator|MakeRotator (+ _roll 1.0) _pitch _yaw) false false))

(event EventBeginPlay
  (switch Utilities|FlowControl|Switch|SwitchonEMagnetPole (Variables|Default|GetMagnetPole)
    (:NewEnumerator0
      (Rendering|Material|SetMaterial (Variables|Default|GetStaticMesh) 0 "/Game/Assets/Object/MI_NorthCore.MI_NorthCore"))
    (:NewEnumerator1
      (Rendering|Material|SetMaterial (Variables|Default|GetStaticMesh) 0 "/Game/Assets/Object/MI_SouthCore.MI_SouthCore")))
  (|CallParentFunction))

(event EventMagnetInteract
  (params (Player%20Magnet%20Pole :type EMagnetPole%20Enum :default "NewEnumerator0") (Player :type Actor%20Object%20Reference) (Player%20Chara%20Movement :type Character%20Movement%20Component%20Object%20Reference) (Delta%20Time :type Float%20%28double-precision%29))
  (bind _self self)
  (bind _staticmesh (Variables|Default|GetStaticMesh))
  (bind _returnvalue (Transformation|GetRelativeTransform _staticmesh))
  (bind _returnvalue_2 (Transformation|GetActorLocation _self))
  (bind _scale (Math|Transform|BreakTransform _returnvalue))
  (bind (_x _y _z) (Math|Vector|BreakVector _scale))
  (bind _returnvalue_3 (Collision|BoxTraceByChannel _returnvalue_2 (+ _returnvalue_2 (* (Transformation|GetActorForwardVector self) (Variables|Default|GetInteract%20Length))) (Math|Vector|MakeVector _x (* _y 50) (* _z 50)) (Transformation|GetActorRotation self) "TraceTypeQuery4" false 0 "ForOneFrame"))
  (if _returnvalue_3
    (Physics|AddForce Player%20Chara%20Movement (* (CallFunction|GetXVector self (CallFunction|IsMagnetPoleEqual Player%20Magnet%20Pole) (Variables|Default|GetRepulsive%20Force) (Variables|Default|GetAttractive%20Force)) -1))))

(fn ConstructionScript)