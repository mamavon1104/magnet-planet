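; Actor that drives screen fade-in and fade-out on a fade widget's image, which it references but does not create.
; FadeIn shows the image and plays a timeline into SetFadeIn; FadeOut reverses a second timeline into SetFadeOut, then makes the image HitTestInvisible.
; On BeginPlay, a one-shot GameInstance flag triggers FadeOut and is cleared; otherwise the fade-out timeline's time is reset and reversed.
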(event Custom|FadeOut
  (Utilities|IsValid (Variables|Default|GetWBP_FadeActor)
    (:Is%20Valid
      (bind _alpha (Timeline|タイムライン_0 ReverseFromEnd)
        (:Update
          (Default|SetFadeOut (Variables|Default|GetWBP_FadeActor) _alpha))
        (:Finished
          (Widget|SetVisibility (Variables|/Game/Characters/BluePrint/UI/WBP_FadeIMage.WBP_FadeIMage_C|GetFadeImage (Variables|Default|GetWBP_FadeActor)) "HitTestInvisible"))))))

(event Custom|FadeIn
  (Utilities|IsValid (Variables|Default|GetWBP_FadeActor)
    (:Is%20Valid
      (Widget|SetVisibility (Variables|/Game/Characters/BluePrint/UI/WBP_FadeIMage.WBP_FadeIMage_C|GetFadeImage (Variables|Default|GetWBP_FadeActor)) "Visible")
      (bind _alpha (Timeline|タイムライン PlayFromStart)
        (:Update
          (Default|SetFadein (Variables|Default|GetWBP_FadeActor) _alpha))))))

(event EventBeginPlay
  (bind _asbp_game_instance (Utilities|Casting|CastToBP_GameINstance (Game|GetGameInstance)))
  (if (Variables|/Game/Game/BP_GameINstance.BP_GameINstance_C|GetIs%20Enabled%20Fade%20Image _asbp_game_instance)
    (Variables|/Game/Game/BP_GameINstance.BP_GameINstance_C|SetIs%20Enabled%20Fade%20Image _asbp_game_instance false)
    (CallFunction|FadeOut)
    (else
      (Utilities|FlowControl|Sequence
        (:then_0
          (bind _alpha (Timeline|タイムライン_0 SetNewTime)
            (:Update
              (Default|SetFadeOut (Variables|Default|GetWBP_FadeActor) _alpha))
            (:Finished
              (Widget|SetVisibility (Variables|/Game/Characters/BluePrint/UI/WBP_FadeIMage.WBP_FadeIMage_C|GetFadeImage (Variables|Default|GetWBP_FadeActor)) "HitTestInvisible"))))
        (:then_1
          (Timeline|タイムライン_0 Reverse))))))

(fn ConstructionScript)