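; Overlap trigger for the magnet character that, judging by its name and debug text, starts a navigation display and camera move when entered.
; ActorBeginOverlap filters for BP_MagnetCharacter, checks an IsDoOnce flag with a DoOnce node and forwards to the parent's overlap handler.
; It then passes the character's BP_PlayerController to the OnTriggerPlayer dispatcher and prints a debug message.
; No camera or drawing logic lives in this Blueprint itself.
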(event EventBeginPlay)

(event Collision|EventActorBeginOverlap
  (params (OtherActor :type Actor%20Object%20Reference))
  (bind _asbp_magnet_character (Utilities|Casting|CastToBP_MagnetCharacter OtherActor))
  (if (Variables|Default|GetIs%20Do%20Once)
    (Utilities|FlowControl|DoOnce false
      (:Completed
        _)))
  (|CallParentFunction _asbp_magnet_character)
  (bind _asbp_player_controller (Utilities|Casting|CastToBP_PlayerController (Pawn|GetController _asbp_magnet_character)))
  (Default|CallOnTriggerPlayer self _asbp_player_controller)
  (Development|PrintString "エリアに入ったのでカメラ移動"))

(event EventTick
  (params (DeltaSeconds :type Float%20%28single-precision%29))
  (|CallParentFunction DeltaSeconds) ; このノードは無効になっているため呼び出せません。\n機能をビルドするにはピンをドラッグしてください。
)

(fn ConstructionScript
  (|CallParentFunction))