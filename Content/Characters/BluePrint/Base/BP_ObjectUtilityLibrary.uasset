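; Blueprint utility library of vector and distance helpers for interactions between the player and objects.
; GetDistanceToPlayer returns a force-sized vector, not a distance: the normalized object-to-player direction, heavily scaled by one of two force inputs.
; The IsObjectToPlayer flag selects that input and, when true, negates the vector.
; Two IsDistanceNotOver checks test whether two positions or actors lie within a given distance, inclusive.
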(fn GetDistancetoPlayer
  (params (Player%20Actor :type Actor%20Object%20Reference) (Object%20Actor :type Actor%20Object%20Reference) (Is%20Object%20To%20Player :type Boolean) (To%20Object%20%20Force :type Float%20%28double-precision%29) (To%20Player%20Force :type Float%20%28double-precision%29))
  (bind _returnvalue (Transformation|GetActorLocation Object%20Actor))
  (bind _returnvalue_2 (Transformation|GetActorLocation Player%20Actor))
  (bind _returnvalue_3 (- _returnvalue_2 _returnvalue))
  (bind _returnvalue_4 (Math|Vector|Normalize _returnvalue_3))
  ;[0.624 0.4912 0.05767 0.5] (プレイヤー - オブジェクト)距離を正規化
  (if Is%20Object%20To%20Player
    ;[0.1226 0.9615 0 0.5] True処理の場合は オブジェクト→プレイヤー
    (return (* _returnvalue_4 -100000 To%20Object%20%20Force))
    (else
      ;[0.9615 0.04563 0 0.5] False処理の場合は プレイヤー→オブジェクト
      (return (* To%20Player%20Force 100000 _returnvalue_4)))))

(fn IsDistanceNotOverPos
  (params (Object%201 :type Vector) (Object2 :type Vector) (Distance :type Integer))
  ;[0.15 0.15 0.15 0.5] 2つのオブジェクトの距離を求めて Distance以内だったらtrueを返す
  (return (<= (Math|Vector|Distance(Vector) Object%201 Object2) Distance)))

(fn IsDistanceNotOverActor
  (params (Object%201 :type Actor%20Object%20Reference) (Object2 :type Actor%20Object%20Reference) (Distance :type Integer))
  ;[0.15 0.15 0.15 0.5] 2つのオブジェクトの距離を求めて Distance以内だったらtrueを返す
  (return (<= (Math|Vector|Distance(Vector) (Transformation|GetActorLocation Object%201) (Transformation|GetActorLocation Object2)) Distance)))