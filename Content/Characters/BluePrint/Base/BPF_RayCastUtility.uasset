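; Utility set of forward ray-cast functions that trace from an actor's root or a camera along its facing direction.
; Line variants return a single Visibility hit, while camera box and sphere variants return multiple hits, each with a hit flag.
; The sphere sweep starts one diameter ahead of the camera and uses TraceTypeQuery3 instead of Visibility.
; All traces leave debug drawing on, and the hit-name print loops are disconnected.
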(fn ForwardLineRayCast(Actor)
  (params (Line%20Cast%20Length :type Integer) (RayActor :type Actor%20Object%20Reference))
  (bind _rootcomponent (Variables|/Script/Engine.Actor|GetRootComponent RayActor))
  (bind _returnvalue (Transformation|GetWorldLocation _rootcomponent))
  (bind (_outhit _returnvalue_2) (Collision|LineTraceByChannel 0 _returnvalue (+ (* Line%20Cast%20Length (Math|Vector|GetForwardVector _rootcomponent)) _returnvalue) "TraceTypeQuery1" false 0 "ForDuration"))
  (return _outhit _returnvalue_2))

(fn ForwardLineRayCast(Camera)
  (params (Line%20Cast%20Length :type Integer) (RayCamera :type Camera%20Component%20Object%20Reference))
  (bind _returnvalue (Transformation|GetWorldLocation RayCamera))
  (bind (_outhit _returnvalue_2) (Collision|LineTraceByChannel 0 _returnvalue (+ (* Line%20Cast%20Length (Math|Vector|GetForwardVector RayCamera)) _returnvalue) "TraceTypeQuery1" false 0 "ForDuration" true "(R=1.000000,G=0.000000,B=0.063861,A=1.000000)" "(R=0.000000,G=1.000000,B=0.103377,A=1.000000)" 2.0))
  (return _outhit _returnvalue_2))

(fn ForwardBoxRayCast(Camera)
  (params (Sphere%20Cast%20Length :type Integer) (RayCamera :type Camera%20Component%20Object%20Reference))
  (bind _returnvalue (Math|Vector|GetForwardVector RayCamera))
  (bind _returnvalue_2 (Transformation|GetWorldLocation RayCamera))
  (bind _returnvalue_3 (* Sphere%20Cast%20Length _returnvalue))
  (bind _returnvalue_4 (+ _returnvalue_3 _returnvalue_2))
  (bind (_outhits _returnvalue_5) (Class|KismetSystemLibrary|BoxTraceMulti 0 _returnvalue_2 _returnvalue_4 (LocalVariables|GetBoxSize) "0, 0, 0" "TraceTypeQuery1" false 0 "ForDuration" true "(R=1.000000,G=0.838378,B=0.000000,A=1.000000)" "(R=0.000000,G=1.000000,B=0.000000,A=1.000000)" 1.0))
  (Rendering|Debug|DrawDebugLine 0 _returnvalue_4 _returnvalue_2 "(R=0.000000,G=0.098495,B=1.000000,A=1.000000)" 1.0)
  (return _outhits _returnvalue_5))

(fn ForwardSphereRayCast(Camera)
  (params (Sphere%20Cast%20Length :type Integer) (RayCamera :type Camera%20Component%20Object%20Reference))
  (bind _returnvalue (Math|Vector|GetForwardVector RayCamera))
  (bind _returnvalue_2 (Transformation|GetWorldLocation RayCamera))
  (bind _sphere_radius (LocalVariables|GetSphere%20Radius))
  (bind _returnvalue_3 (* Sphere%20Cast%20Length _returnvalue))
  (bind _returnvalue_4 (* _returnvalue _sphere_radius 2.0))
  (bind _returnvalue_5 (+ _returnvalue_4 _returnvalue_2))
  (bind _returnvalue_6 (+ _returnvalue_3 _returnvalue_2))
  (bind (_outhits _returnvalue_7) (Collision|MultiSphereTraceByChannel 0 _returnvalue_5 _returnvalue_6 (LocalVariables|GetSphere%20Radius) "TraceTypeQuery3" false 0 "ForDuration" true "(R=1.000000,G=0.000000,B=0.000000,A=1.000000)" "(R=0.000000,G=1.000000,B=0.000000,A=1.000000)" 1.0))
  (Rendering|Debug|DrawDebugLine 0 _returnvalue_5 _returnvalue_6 "(R=0.000000,G=0.098495,B=1.000000,A=1.000000)" 1.0)
  (return _outhits _returnvalue_7))