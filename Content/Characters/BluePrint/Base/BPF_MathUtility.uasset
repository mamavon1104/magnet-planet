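; Blueprint function library of math helpers for character Blueprints.
; Plus-equal and minus-equal functions for float and int modify a by-ref variable in place and return the result.
; A targeting helper normalizes the direction from a self actor to a target actor and returns its dot and cross products with the self actor's forward vector.
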(fn PlusEqualFunction(Float)
  (params (Value :type Float%20%28double-precision%29%20%28by%20ref%29) (AddValue :type Float%20%28double-precision%29))
  (|SetBy-RefVar Value (+ Value AddValue))
  (return Value))

(fn PlusEqualFunction(Int)
  (params (Value :type Integer%20%28by%20ref%29) (AddValue :type Integer))
  (|SetBy-RefVar Value (+ Value AddValue))
  (return Value))

(fn MinusEqualFunction(Int)
  (params (Value :type Integer%20%28by%20ref%29) (SubtractValue :type Integer) (__WorldContext :type Object%20Object%20Reference))
  (|SetBy-RefVar Value (- Value SubtractValue))
  (return Value))

(fn MinusEqualFunction(Float)
  (params (Value :type Float%20%28double-precision%29%20%28by%20ref%29) (SubtractValue :type Float%20%28double-precision%29) (__WorldContext :type Object%20Object%20Reference))
  (|SetBy-RefVar Value (- Value SubtractValue))
  (return Value))

(fn GetTargetandForwardDotCross(Actor)
  (params (Target%20Actor :type Actor%20Object%20Reference) (Self%20Actor :type Actor%20Object%20Reference))
  (bind _returnvalue (Transformation|GetActorForwardVector Self%20Actor))
  (bind _returnvalue_2 (Transformation|GetActorLocation Self%20Actor))
  (bind _returnvalue_3 (Transformation|GetActorLocation Target%20Actor))
  (bind _returnvalue_4 (- _returnvalue_3 _returnvalue_2))
  (bind _returnvalue_5 (Math|Vector|Normalize _returnvalue_4))
  ;[0.15 0.15 0.15 0.5] ターゲットへの正規化ベクトルと前方ベクトルで内積と外積を求める
  (return (Math|Vector|DotProduct _returnvalue_5 _returnvalue) (Math|Vector|CrossProduct _returnvalue_5 _returnvalue)))