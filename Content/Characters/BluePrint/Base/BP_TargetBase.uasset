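; Base Blueprint for a magnetic target with a core and ring that animate by pole and interaction state.
; Looping timers replay Timelines for idle counter-rotation, swapped for a selected animation between ray hit and miss events.
; ReversePole pauses both timers and plays a fast core spin, forward or backward by pole.
; An event track mid-spin calls the parent's reversal and swaps the core mesh and red/blue ring material.
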(event Custom|HitRayEvent
  ;[0 0.6406 0.07106 0.5] インタラクト可能になったらアニメーションタイマーを別に起動して、そっちからアニメーションさせる
  (Utilities|FlowControl|Sequence
    (:then_0
      ;[0.15 0.15 0.15 0.5] ゲーム開始されたら３秒間のタイマーを起動して、タイムラインから alpha値を取得して0~360のZ回転を実行しています。
      (bind _rotation_alpha (Timeline|Natural%20Rotate%20Animation Stop)
        (:Update
          (Transformation|SetRelativeRotation (Variables|Default|GetStaticMesh) (Math|Rotator|CombineRotators (Variables|Default|GetStartCoreRotator) (Math|Rotator|Lerp(Rotator) "0, 0, 0" "0.000000,540.000000,0.000000" _rotation_alpha)) false false)
          (Transformation|SetRelativeRotation (Variables|Default|GetRingMesh) (Math|Rotator|CombineRotators (Variables|Default|GetStartRingRotator) (* (Math|Rotator|CombineRotators (Variables|Default|GetStartCoreRotator) (Math|Rotator|Lerp(Rotator) "0, 0, 0" "0.000000,540.000000,0.000000" _rotation_alpha)) -1)) false false))))
    (:then_1
      (Class|KismetSystemLibrary|PauseTimer 0 "Repeate Rotate Anime"))
    (:then_2
      (Utilities|Time|SetTimerbyEvent (delegate Custom|Repeate%20SelectedAnim) 4.0 true false -4.0))))

(event Custom|MissRayEvent
  ;[0.15 0 0 0.5] インタラクト不可能になった場合、タイマーを再開して自分のアニメーションをこの一回(NumLoops : 0)で停止させる
  (Utilities|FlowControl|Sequence
    (:then_0
      ;[0 0.6406 0.07106 0.5] インタラクト可能になったらアニメーションタイマーを別に起動して、そっちからアニメーションさせる
      (bind (_direction _corerotate _ringrotate) (Timeline|HitEvent Stop)
        (:Update
          (Transformation|SetRelativeRotation (Variables|Default|GetStaticMesh) (Math|Rotator|CombineRotators (Variables|Default|GetStartCoreRotator) (CallFunction|CreateRotatorfromVector _corerotate)) false false)
          (Transformation|SetRelativeRotation (Variables|Default|GetRingMesh) (Math|Rotator|CombineRotators (Variables|Default|GetStartRingRotator) (CallFunction|CreateRotatorfromVector _ringrotate)) false false))))
    (:then_1
      (Class|KismetSystemLibrary|PauseTimer 0 "Repeate SelectedAnim")
      (Class|KismetSystemLibrary|UnPauseTimer 0 "Repeate Rotate Anime")
      (CallFunction|ResetNaturalRotateTImer))))

(event Custom|Repeate%20Rotate%20Anime
  ;[0.15 0.15 0.15 0.5] ゲーム開始されたら３秒間のタイマーを起動して、タイムラインから alpha値を取得して0~360のZ回転を実行しています。
  (bind _rotation_alpha (Timeline|Natural%20Rotate%20Animation PlayFromStart)
    (:Update
      (Transformation|SetRelativeRotation (Variables|Default|GetStaticMesh) (Math|Rotator|CombineRotators (Variables|Default|GetStartCoreRotator) (Math|Rotator|Lerp(Rotator) "0, 0, 0" "0.000000,540.000000,0.000000" _rotation_alpha)) false false)
      (Transformation|SetRelativeRotation (Variables|Default|GetRingMesh) (Math|Rotator|CombineRotators (Variables|Default|GetStartRingRotator) (* (Math|Rotator|CombineRotators (Variables|Default|GetStartCoreRotator) (Math|Rotator|Lerp(Rotator) "0, 0, 0" "0.000000,540.000000,0.000000" _rotation_alpha)) -1)) false false))))

(event Custom|Repeate%20SelectedAnim
  ;[0 0.6406 0.07106 0.5] インタラクト可能になったらアニメーションタイマーを別に起動して、そっちからアニメーションさせる
  (bind (_direction _corerotate _ringrotate) (Timeline|HitEvent PlayFromStart)
    (:Update
      (Transformation|SetRelativeRotation (Variables|Default|GetStaticMesh) (Math|Rotator|CombineRotators (Variables|Default|GetStartCoreRotator) (CallFunction|CreateRotatorfromVector _corerotate)) false false)
      (Transformation|SetRelativeRotation (Variables|Default|GetRingMesh) (Math|Rotator|CombineRotators (Variables|Default|GetStartRingRotator) (CallFunction|CreateRotatorfromVector _ringrotate)) false false))))

(event Custom|Reset%20Natural%20Rotate%20TImer
  ;[0.15 0.15 0.15 0.5] ゲーム開始されたら３秒間のタイマーを起動して、タイムラインから alpha値を取得して0~360のZ回転を実行しています。
  (Utilities|Time|SetTimerbyEvent (delegate Custom|Repeate%20Rotate%20Anime) 4.0 true false -4.0)
  ;[0.15 0.15 0.15 0.5] 極によってマテリアルを変える(SM_Ring)
  ; 極変更の場合はコアスタティックメッシュも変更するよ
  (switch Utilities|FlowControl|Switch|SwitchonEMagnetPole (Variables|Default|GetMagnetPole)
    (:NewEnumerator0
      (Rendering|Material|SetMaterial (Variables|Default|GetRingMesh) 0 "/Game/Assets/Object/MI_RedRing.MI_RedRing"))
    (:NewEnumerator1
      (Rendering|Material|SetMaterial (Variables|Default|GetRingMesh) 0 "/Game/Assets/Object/MI_RingBlue.MI_RingBlue")))
  (|CallParentFunction))

(event Custom|Change%20Pole%20Material%20And%20Mesh
  ;[0.15 0.15 0.15 0.5] ゲーム開始されたら３秒間のタイマーを起動して、タイムラインから alpha値を取得して0~360のZ回転を実行しています。
  (Components|StaticMesh|SetStaticMesh (Variables|Default|GetStaticMesh) (Variables|Default|GetNext%20Core%20StaticMesh))
  ;[0.15 0.15 0.15 0.5] 極によってマテリアルを変える(SM_Ring)
  ; 極変更の場合はコアスタティックメッシュも変更するよ
  (switch Utilities|FlowControl|Switch|SwitchonEMagnetPole (Variables|Default|GetMagnetPole)
    (:NewEnumerator0
      (Rendering|Material|SetMaterial (Variables|Default|GetRingMesh) 0 "/Game/Assets/Object/MI_RedRing.MI_RedRing"))
    (:NewEnumerator1
      (Rendering|Material|SetMaterial (Variables|Default|GetRingMesh) 0 "/Game/Assets/Object/MI_RingBlue.MI_RingBlue")))
  (|CallParentFunction))

(event EventBeginPlay
  ;[0.15 0.15 0.15 0.5] ゲーム開始されたら３秒間のタイマーを起動して、タイムラインから alpha値を取得して0~360のZ回転を実行しています。
  (Utilities|FlowControl|Sequence
    (:then_0
      (Variables|Default|SetStartCoreRotator (Transformation|GetActorRotation self))
      (Variables|Default|SetStartRingRotator (Transformation|GetWorldRotation (Variables|Default|GetRingMesh)))
      (Utilities|Time|SetTimerbyEvent (delegate Custom|Repeate%20Rotate%20Anime) 4.0 true false -4.0)
      ;[0.15 0.15 0.15 0.5] 極によってマテリアルを変える(SM_Ring)
      ; 極変更の場合はコアスタティックメッシュも変更するよ
      (switch Utilities|FlowControl|Switch|SwitchonEMagnetPole (Variables|Default|GetMagnetPole)
        (:NewEnumerator0
          (Rendering|Material|SetMaterial (Variables|Default|GetRingMesh) 0 "/Game/Assets/Object/MI_RedRing.MI_RedRing"))
        (:NewEnumerator1
          (Rendering|Material|SetMaterial (Variables|Default|GetRingMesh) 0 "/Game/Assets/Object/MI_RingBlue.MI_RingBlue")))
      (|CallParentFunction))))

(event EventReversePole
  ;[0.15 0.15 0.15 0.5] マグネットの極を変える時にくるくる回転させるアニメーションにしたいんです
  ; Blenderで粘ってAnimationにしなかったことを物凄く後悔しています本当にです。次のゲームから気を付けましょう
  (Utilities|FlowControl|Sequence
    (:then_0
      (switch Utilities|FlowControl|Switch|SwitchonEMagnetPole (Variables|Default|GetMagnetPole)
        (:NewEnumerator0
          (bind _rotation_alpha (Timeline|Change%20Rotate%20Animation PlayFromStart)
            (:Update
              (Transformation|SetRelativeRotation (Variables|Default|GetStaticMesh) (Math|Rotator|CombineRotators (Variables|Default|GetStartCoreRotator) (Math|Rotator|Lerp(Rotator) "0, 0, 0" "0.000000,3240.000000,0.000000" _rotation_alpha)) false false))
            (:Finished
              (Class|KismetSystemLibrary|UnPauseTimer 0 "Repeate Rotate Anime")
              (Class|KismetSystemLibrary|UnPauseTimer 0 "Repeate SelectedAnim"))
            (:Reverse%20Pole%20Event%20Timing
              (|CallParentFunction)
              (CallFunction|ChangePoleMaterialandMesh))))
        (:NewEnumerator1
          (Timeline|Change%20Rotate%20Animation ReverseFromEnd))))
    (:then_1
      (Class|KismetSystemLibrary|PauseTimer 0 "Repeate SelectedAnim"))
    (:then_2
      (Class|KismetSystemLibrary|PauseTimer 0 "Repeate Rotate Anime"))))

(fn ConstructionScript
  (|CallParentFunction))