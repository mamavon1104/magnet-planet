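; Pedestal that captures a BP_FollowActor and turns magnet interaction with it into a 0–1 alpha.
; A 0.5s timer snaps the cursor pivot in 90° steps toward the player's side using dot/cross products, and box-traces for a follow actor.
; A found actor stops being interactable, passes on its pole, and eases into a socket via timeline.
; MagnetInteract spins it by pole match, raising or lowering the clamped timer behind CallChangeAlphaEvent.
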(event Custom|Check%20Is%20Hit%20Ray%20Cast
  (bind _self self)
  (bind _player (Variables|Default|GetPlayer))
  (bind (_dot _cross) (CallFunction|GetTargetandForwardDotCross(Actor) _player _self))
  (bind _returnvalue (Class|KismetMathLibrary|DegAcos _dot))
  ;[0 0.7406 0.4727 0.5 64] 0.5秒ごとにカーソルの位置を変更する処理
  (Utilities|FlowControl|Sequence
    (:then_0
      (Utilities|IsValid (Variables|Default|GetPlayer)
        (:Is%20Valid
          ;;[0.15 0.15 0.15 0.5] 前後左右何処にいるか判定して、カーソルを90℃ずつ回転させる仕組み
          (if (<= _returnvalue 45.0)
            ;;;[0.15 0.15 0.15 0.5] 45度以下だったら
            (Transformation|SetRelativeRotation (Variables|Default|GetCursor%20Pivot) "0.000000,180.000000,0.000000" false false)
            (elif (<= _returnvalue 135.0)
              ;;;[0.15 0.15 0.15 0.5] zベクトルの外積結果で左右か確認
              (if (> (.Z (Math|Vector|BreakVector _cross)) 0.0)
                ;;;[0.15 0.15 0.15 0.5] 右の場合
                (Transformation|SetRelativeRotation (Variables|Default|GetCursor%20Pivot) "0.000000,90.000000,0.000000" false false)
                (else
                  ;;;[0.15 0.15 0.15 0.5] 左の場合
                  (Transformation|SetRelativeRotation (Variables|Default|GetCursor%20Pivot) "0.000000,270.000000,0.000000" false false)))
              (else
                ;;;[0.15 0.15 0.15 0.5] 135度以上だったら
                (Transformation|SetRelativeRotation (Variables|Default|GetCursor%20Pivot) "0, 0, 0" false false)))))))
    (:then_1
      ;;[0.1426 0 1 0.5] FollowActorがこの台座の範囲内にいるかどうかの判定
      (Utilities|IsValid (Variables|Default|GetFollow%20Actor)
        (:Is%20Not%20Valid
          (bind (_outhit _returnvalue_2) (Collision|BoxTraceByChannel (Transformation|GetWorldLocation (Variables|Default|GetStaticMesh)) (Transformation|GetWorldLocation (Variables|Default|GetEndPoint)) "420.000000,420.000000,1.000000" "0, 0, 0" "TraceTypeQuery3" false 0 "ForDuration" true "(R=1.000000,G=0.000000,B=0.000000,A=1.000000)" "(R=0.000000,G=1.000000,B=0.000000,A=1.000000)" 0.5))
          (if _returnvalue_2
            (Development|PrintString (Utilities|GetDisplayName (.HitActor (Collision|BreakHitResult _outhit))))
            (bind _asbp_follow_actor (Utilities|Casting|CastToBP_FollowActor (.HitActor (Collision|BreakHitResult _outhit))))
            (Variables|Default|SetFollow%20Actor _asbp_follow_actor)
            (Variables|/Game/Characters/BluePrint/Base/BP_MagnetInteractableBase.BP_MagnetInteractableBase_C|SetCan%20Interact _asbp_follow_actor false)
            (Default|OnPlacedonFollowStand _asbp_follow_actor)
            (Variables|Default|SetMagnetPole (Variables|/Game/Characters/BluePrint/Base/BP_MagnetInteractableBase.BP_MagnetInteractableBase_C|GetMagnetPole _asbp_follow_actor))
            (bind _alpha (Timeline|Set%20Follow%20Actor%20Position Play)
              (:Update
                (Utilities|FlowControl|Sequence
                  (:then_0
                    (Transformation|SetActorLocation (Variables|Default|GetFollow%20Actor) (Math|Vector|Lerp(Vector) (Transformation|GetActorLocation _asbp_follow_actor) (Transformation|GetSocketLocation (Variables|Default|GetStaticMesh) "FollowActorSocket") _alpha) false false)
                    (Development|PrintString (Utilities|String|ToString(Vector) (Math|Vector|Lerp(Vector) (Transformation|GetActorLocation _asbp_follow_actor) (Transformation|GetSocketLocation (Variables|Default|GetStaticMesh) "FollowActorSocket") _alpha))))
                  (:then_1
                    (Transformation|SetActorRotation (Variables|Default|GetFollow%20Actor) (Class|KismetMathLibrary|QuatRotator (Class|KismetMathLibrary|QuatSlerp (Math|Conversions|ToQuaternion(Rotator) (Transformation|GetActorRotation _asbp_follow_actor)) (Math|Conversions|ToQuaternion(Rotator) (Transformation|GetSocketRotation (Variables|Default|GetStaticMesh) "FollowActorSocket")) _alpha)))
                    (Development|PrintString (Utilities|String|ToString(Rotator) (Class|KismetMathLibrary|QuatRotator (Class|KismetMathLibrary|QuatSlerp (Math|Conversions|ToQuaternion(Rotator) (Transformation|GetActorRotation _asbp_follow_actor)) (Math|Conversions|ToQuaternion(Rotator) (Transformation|GetSocketRotation (Variables|Default|GetStaticMesh) "FollowActorSocket")) _alpha))))))))))))))

(event EventBeginPlay
  ;[0 0.7406 0.4727 0.5 64] 0.5秒ごとにカーソルの位置を変更する処理
  (Utilities|Time|SetTimerbyEvent (delegate Custom|Check%20Is%20Hit%20Ray%20Cast) 0.5 true)
  (|CallParentFunction))

(event EventMagnetInteract
  (params (Player%20Magnet%20Pole :type EMagnetPole%20Enum :default "NewEnumerator0") (Player :type Actor%20Object%20Reference) (Player%20Chara%20Movement :type Character%20Movement%20Component%20Object%20Reference) (Delta%20Time :type Float%20%28double-precision%29))
  (bind _follow_actor (Variables|Default|GetFollow%20Actor))
  (bind _returnvalue (Transformation|GetActorRotation _follow_actor))
  (bind (_roll _pitch _yaw) (Math|Rotator|BreakRotator _returnvalue))
  (bind (_roll_2 _pitch_2 _yaw_2) (Math|Rotator|BreakRotator _returnvalue))
  ;[0.15 0.15 0.15 0.5 25] インタラクトが　初めてならプレイヤーをセット、その後のフレームから alpha 変更を開始 タイマーを変更してその値を制限、割って0~1で算出)
  ; インタラクトされてる間はMakeRotatorで回転させる。
  (Utilities|IsValid (Variables|Default|GetPlayer)
    (:Is%20Valid
      (Utilities|IsValid (Variables|Default|GetFollow%20Actor)
        (:Is%20Valid
          (if (CallFunction|IsMagnetPoleEqual Player%20Magnet%20Pole)
            (Transformation|SetActorRotation (Variables|Default|GetFollow%20Actor) (Math|Rotator|MakeRotator _roll_2 _pitch_2 (+ _yaw_2 (Variables|Default|GetFollow%20Actor%20Rotate%20Speed))))
            ;;[0 0.874 0.225 0.5] 値を加算して0~1のalpha値を算出
            (CallFunction|PlusEqualFunction(Float) (Variables|Default|GetInteract%20Timer) Delta%20Time)
            (else
              (Transformation|SetActorRotation (Variables|Default|GetFollow%20Actor) (Math|Rotator|MakeRotator _roll _pitch (- _yaw (Variables|Default|GetFollow%20Actor%20Rotate%20Speed))))
              (CallFunction|MinusEqualFunction(Float) (Variables|Default|GetInteract%20Timer) Delta%20Time)))
          (bind _output_get (Variables|Default|SetInteract%20Timer (Math|Float|Clamp(Float) (Variables|Default|GetInteract%20Timer) 0.0 (Variables|Default|GetMax%20Interact%20Time))))
          (Default|CallChangeAlphaEvent self (/ _output_get (Variables|Default|GetMax%20Interact%20Time))))))
    (:Is%20Not%20Valid
      (Variables|Default|SetPlayer Player))))

(fn ConstructionScript
  (|CallParentFunction))