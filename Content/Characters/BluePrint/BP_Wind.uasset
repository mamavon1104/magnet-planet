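; BP_Wind is a wind volume that pushes the magnet character and falling blocks along its StartPoint-to-EndPoint direction.
; Overlap events store the character's movement component and track other actors in WindowObjects, though their Contains checks test the failed cast result.
; Tick applies distance-scaled force to each BP_FallBlock mesh.
; A per-tick DoOnce inside that loop pushes the player once, only when the list is non-empty.
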(event EventTick
  (params (DeltaSeconds :type Float%20%28single-precision%29))
  (bind _startpoint (Variables|Default|GetStartPoint))
  (bind _endpoint (Variables|Default|GetEndPoint))
  (bind _playercharactermovement (Variables|Default|GetPlayerCharacterMovement))
  (bind _returnvalue (Transformation|GetWorldLocation _startpoint))
  (bind _returnvalue_2 (Transformation|GetWorldLocation _endpoint))
  (bind _returnvalue_3 (- _returnvalue_2 _returnvalue))
  (bind _returnvalue_4 (* _returnvalue_3 200))
  ;[0.15 0.15 0.15 0.5] Tick内で(Start → End) × WindPowerの力だけWindowObjectsに力を加える(CharacterMovementは一度だけ実行する為DoOnce)
  (for _array_element (Variables|Default|GetWindowObjects)
    (Utilities|FlowControl|Sequence
      (:then_0
        (Utilities|FlowControl|DoOnce false
          (:Completed
            (Utilities|IsValid _playercharactermovement
              (:Is%20Valid
                (Physics|AddForce _playercharactermovement _returnvalue_4))))))
      (:then_1
        (bind _asbp_fall_block (Utilities|Casting|CastToBP_FallBlock _array_element))
        (Physics|AddForce (Variables|/Game/Characters/BluePrint/BP_FallBlock.BP_FallBlock_C|GetStaticMesh _asbp_fall_block) _returnvalue_4 "None" false))))
  (Utilities|FlowControl|DoOnce false) ; enters at Reset
)

(event Collision|EventActorBeginOverlap
  (params (OtherActor :type Actor%20Object%20Reference))
  ;[0.15 0.15 0.15 0.5] トリガーに出入りしたらCharacterMovementを取得。
  (bind _asbp_magnet_character (Utilities|Casting|CastToBP_MagnetCharacter OtherActor)
    (:then
      (Variables|Default|SetPlayerCharacterMovement (Variables|/Script/Engine.Character|GetCharacterMovement _asbp_magnet_character)))
    (:CastFailed
      (if (not (Utilities|Array|ContainsItem (Variables|Default|GetWindowObjects) _asbp_magnet_character))
        (Utilities|Array|Add (Variables|Default|GetWindowObjects) OtherActor)))))

(event Collision|EventActorEndOverlap
  (params (OtherActor :type Actor%20Object%20Reference))
  ;[0.15 0.15 0.15 0.5] トリガーに出入りしたらCharacterMovementを取得。
  (bind _asbp_magnet_character (Utilities|Casting|CastToBP_MagnetCharacter OtherActor)
    (:then
      (Variables|Default|SetPlayerCharacterMovement 0))
    (:CastFailed
      (if (Utilities|Array|ContainsItem (Variables|Default|GetWindowObjects) _asbp_magnet_character)
        (Utilities|Array|RemoveItem (Variables|Default|GetWindowObjects) OtherActor)))))

(fn ConstructionScript)