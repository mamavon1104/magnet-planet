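; BP_SwingBase is a magnet-polarity swing actor whose Ring is colored to show its pole.
; On BeginPlay it switches on MagnetPole, giving Ring a red material for North or a blue one for South, then calls the parent BeginPlay.
; No swing logic runs in this graph: overlap and Tick are disabled, the timeline is unconnected and IsSelect is unused.
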(event EventBeginPlay
  (switch Utilities|FlowControl|Switch|SwitchonEMagnetPole (Variables|Default|GetMagnetPole)
    (:NewEnumerator0
      (Rendering|Material|SetMaterial (Variables|Default|GetRing) 0 "/Game/Assets/Object/MI_RedRing.MI_RedRing"))
    (:NewEnumerator1
      (Rendering|Material|SetMaterial (Variables|Default|GetRing) 0 "/Game/Assets/Object/MI_RingBlue.MI_RingBlue")))
  (|CallParentFunction))

(event Collision|EventActorBeginOverlap
  (params (OtherActor :type Actor%20Object%20Reference))
  (|CallParentFunction OtherActor) ; このノードは無効になっているため呼び出せません。\n機能をビルドするにはピンをドラッグしてください。
)

(event EventTick
  (params (DeltaSeconds :type Float%20%28single-precision%29))
  (|CallParentFunction DeltaSeconds) ; このノードは無効になっているため呼び出せません。\n機能をビルドするにはピンをドラッグしてください。
)

(fn ConstructionScript
  (|CallParentFunction))