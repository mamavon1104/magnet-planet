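; BP_SwingPoint is a magnetic point that pushes or pulls the player through character movement.
; BeginPlay picks a north or south core mesh from its MagnetPole before calling the parent.
; MagnetInteract compares poles, feeds attractive and repulsive forces into GetDistanceToPlayer, and applies the negated result as a force on the player.
; It draws a debug sphere at the release radius, but the commented in-range release is not implemented here.
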(event EventBeginPlay
  (switch Utilities|FlowControl|Switch|SwitchonEMagnetPole (Variables|Default|GetMagnetPole)
    (:NewEnumerator0
      (Components|StaticMesh|SetStaticMesh (Variables|Default|GetStaticMesh) "/Game/Assets/Object/SM_NorthMountainShapeCore.SM_NorthMountainShapeCore"))
    (:NewEnumerator1
      (Components|StaticMesh|SetStaticMesh (Variables|Default|GetStaticMesh) "/Game/Assets/Object/SM_SouthMoutainShapeCore.SM_SouthMoutainShapeCore")))
  (|CallParentFunction))

(event Collision|EventActorBeginOverlap
  (params (OtherActor :type Actor%20Object%20Reference))
  (|CallParentFunction OtherActor) ; このノードは無効になっているため呼び出せません。\n機能をビルドするにはピンをドラッグしてください。
)

(event EventMagnetInteract
  (params (Player%20Magnet%20Pole :type EMagnetPole%20Enum :default "NewEnumerator0") (Player :type Actor%20Object%20Reference) (Player%20Chara%20Movement :type Character%20Movement%20Component%20Object%20Reference))
  ;[0.5729 0.02068 0 0.5] プレイヤーをオブジェクトに引き寄せて、 指定した範囲内ならばプレイヤーの持っているオブジェクトをリリースする
  (Utilities|FlowControl|Sequence
    (:then_0
      (Rendering|Debug|DrawDebugSphere (Transformation|GetActorLocation self) (Math|Conversions|ToFloat(Integer) (Variables|Default|GetRelease%20Sphere%20Radius)) 4 "(R=0.000000,G=0.189954,B=1.000000,A=1.000000)" 0.0))
    (:then_1
      (Physics|AddForce Player%20Chara%20Movement (* (CallFunction|GetDistancetoPlayer Player self (CallFunction|IsMagnetPoleEqual Player%20Magnet%20Pole) (Variables|Default|GetAttractive%20Force) (Variables|Default|GetRepulsive%20Force)) -1)))))

(fn ConstructionScript
  (|CallParentFunction))